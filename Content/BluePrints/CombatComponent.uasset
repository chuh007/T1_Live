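; CombatComponent is an actor component that gives its owner hit points and handles dealing and taking damage.
; HP starts at MaxHp on BeginPlay, and ConbatAttack passes damage to the hit actor's own CombatComponent, if it has one.
; CombatHit subtracts damage with clamping between zero and MaxHp, then calls the OnChangedHP dispatcher, plus OnHpZero when HP reaches zero.
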(event EventBeginPlay
  (Variables|Default|SetHP (Variables|Default|GetMaxHp)))

(event EventTick
  (params (DeltaSeconds :type Float%20%28single-precision%29)))

(fn ConbatAttack
  (params (Damage :type Float%20%28double-precision%29) (HitActor :type Actor%20Object%20Reference))
  (bind _returnvalue (Actor|GetComponentbyClass HitActor "CombatComponent_C"))
  (Utilities|IsValid _returnvalue
    (:Is%20Valid
      (CallFunction|CombatHit _returnvalue Damage))))

(fn CombatHit
  (params (Damage :type Float%20%28double-precision%29))
  (bind _output_get (Variables|Default|SetHP (Math|Float|Clamp(Float) (- (Variables|Default|GetHP) Damage) 0.0 (Variables|Default|GetMaxHp))))
  (Default|CallOnChangedHP _output_get (Variables|Default|GetMaxHp))
  (if (<= (Variables|Default|GetHP) 0.0)
    (Default|CallOnHpZero)))